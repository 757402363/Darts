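; Throwable dart actor that is picked up by attaching to a given component and thrown by detaching with physics on.
; A looping timer started on drop apparently aligns the dart to its velocity and line-traces ahead of the tip for impacts.
; A trace or static-mesh capsule hit freezes the dart, blocks re-pickup and sets a short lifespan.
; An equally long delay precedes the DartThrown call.
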(event OnComponentHit(Capsule)
  (params (HitComponent :type Primitive%20Component%20Object%20Reference) (OtherActor :type Actor%20Object%20Reference) (OtherComp :type Primitive%20Component%20Object%20Reference) (NormalImpulse :type Vector :default "0, 0, 0") (Hit :type Hit%20Result%20Structure%20%28by%20ref%29))
  (Utilities|Casting|CastToStaticMeshActor OtherActor)
  (CallFunction|StopDartMotion))

(event Custom|AdjustRotationFromThrow
  (bind _dart_controller (Variables|Default|GetDart_Controller))
  (Transformation|SetWorldRotation _dart_controller (Math|Rotator|MakeRotfromX (Transformation|GetComponentVelocity _dart_controller)) false false)
  (CallFunction|CheckHitSomething))

(event Custom|CheckHitSomething
  (bind _arrow (Variables|Default|GetArrow))
  (bind _returnvalue (Transformation|GetWorldLocation _arrow))
  (bind _outhit (Collision|LineTraceByChannel _returnvalue (+ _returnvalue (* (Math|Vector|GetForwardVector _arrow) 15.0)) "TraceTypeQuery1" false 0 "None"))
  (if (.bBlockingHit (Collision|BreakHitResult _outhit))
    (CallFunction|StopDartMotion)))

(event Custom|StopDartMotion
  (Physics|SetSimulatePhysics (Variables|Default|GetDart_Controller) false)
  (Utilities|Time|PauseTimerbyHandle (Variables|ControlTimer|GetDartRotationTimer))
  (Actor|SetLifeSpan 3.0)
  (Variables|Default|SetThrownAlready true)
  (Utilities|FlowControl|Delay 3.0)
  (Default|CallDartThrown)
  (Variables|Default|SetThrownAlready false))

(event EventBeginPlay)

(event Collision|EventActorBeginOverlap
  (params (OtherActor :type Actor%20Object%20Reference)))

(event EventTick
  (params (DeltaSeconds :type Float%20%28single-precision%29)))

(event EventPickup
  (params (AttachTo :type Scene%20Component%20Object%20Reference))
  (if (not (Variables|Default|GetThrownAlready))
    (Physics|SetSimulatePhysics (Variables|Default|GetDart_Controller) false)
    (Transformation|AttachComponentToComponent (VehicleSound|GetRootComponent) AttachTo "None" "KeepWorld" "KeepWorld" "KeepWorld" false)))

(event EventDrop
  (Physics|SetSimulatePhysics (Variables|Default|GetDart_Controller) true)
  (Transformation|DetachFromActor "KeepWorld" "KeepWorld" "KeepWorld")
  (bind _returnvalue (Utilities|Time|SetTimerbyEvent (EventDispatchers|CreateEvent :!event Custom|AdjustRotationFromThrow) (/ 1.0 6e+01) true))
  (Variables|ControlTimer|SetDartRotationTimer _returnvalue))

(fn ConstructionScript)