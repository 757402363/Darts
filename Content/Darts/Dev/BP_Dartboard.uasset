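; Dartboard actor for the darts game that detects hits, tracks a rotating bonus quadrant and keeps the player's score.
; Board hits resolve to a quadrant via Atan2 around the Arrow component, then report to GameMode_Darts with a bonus flag.
; A bonus hit randomly picks a different quadrant.
; UpdateScore splits points into standard and bonus totals and feeds the horizontal and vertical widgets, the latter also tracking throws.
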(event Custom|SetNewBonus
  (bind _output_get (Variables|Quadrant|SetPossibleQuadrant (Utilities|Array|MakeArray 1 2 3 4)))
  (Utilities|Array|RemoveItem _output_get (Variables|Quadrant|GetBonusQuadrant))
  (Utilities|Array|Shuffle (Variables|Quadrant|GetPossibleQuadrant))
  (Variables|Quadrant|SetBonusQuadrant (Utilities|Array|Get(acopy) (Variables|Quadrant|GetPossibleQuadrant) (Math|Random|RandomIntegerinRange 0 2))))

(event Custom|DartboardHit
  (params (HitLocation :type Vector) (ComponentHit :type Primitive%20Component%20Object%20Reference))
  (bind _dartboard (Variables|Default|GetDartboard))
  (bind _returnvalue (== ComponentHit _dartboard))
  (Default|UpdateThrows (Variables|Reference|GetW_Darts_Vert) _returnvalue)
  (if _returnvalue
    (bind _quadrant (HitQuadrant|DetermineQuadrantOfHit HitLocation))
    (bind _asgame_mode_darts (Utilities|Casting|CastToGameMode_Darts (Game|GetGameMode)))
    (Default|PlayerHasScored _asgame_mode_darts (== _quadrant (Variables|Quadrant|GetBonusQuadrant)) self)
    (if (== _quadrant (Variables|Quadrant|GetBonusQuadrant))
      (CallFunction|SetNewBonus))))

(event Custom|UpdateScore
  (params (PointsAdded :type Integer) (BonusHit :type Boolean))
  ;[1 1 1] Update the offical score count, seperate it by score type, and send data to Widget
  (bind _output_get (Variables|ScoreData|SetPlayerScore (+ (Variables|ScoreData|GetPlayerScore) PointsAdded)))
  (Default|UpdateScore (Variables|Reference|GetW_Darts_Horiz) _output_get BonusHit)
  (if BonusHit
    (Variables|ScoreData|SetBonusTotal (+ (Variables|ScoreData|GetBonusTotal) PointsAdded))
    (else
      (Variables|ScoreData|SetStandardTotal (+ PointsAdded (Variables|ScoreData|GetStandardTotal)))))
  (Default|UpdateUserScore (Variables|Reference|GetW_Darts_Vert) (Variables|ScoreData|GetBonusTotal) (Variables|ScoreData|GetStandardTotal)))

(event EventBeginPlay
  ;[1 1 1] Reference to the material of the dartboard
  (bind _returnvalue (Rendering|Material|CreateDynamicMaterialInstance (Variables|Default|GetDartboard) 0 0 "None" :!class /Script/Engine.PrimitiveComponent))
  (Variables|Material|SetDartboard_Material _returnvalue)
  (Variables|Reference|SetW_Darts_Horiz (.AsW%20Darts%20Main%20Horiz (Utilities|Casting|CastToW_Darts_Main_Horiz (UserInterface|GetUserWidgetObject (Variables|Default|GetWidget)))))
  (Variables|Reference|SetW_Darts_Vert (.AsW%20Darts%20Main%20Vert (Utilities|Casting|CastToW_Darts_Main_Vert (UserInterface|GetUserWidgetObject (Variables|/Game/Darts/UI/Actors/BP_GameBoardData.BP_GameBoardData_C|GetWidget (Variables|Reference|GetGameboardData))))))
  (CallFunction|SetNewBonus))

(fn ConstructionScript)

(fn DetermineQuadrantOfHit
  (params (HitLocation :type Vector))
  (bind _arrow (Variables|Default|GetArrow))
  (bind _returnvalue (Transformation|GetWorldLocation _arrow))
  (bind _returnvalue_2 (- HitLocation _returnvalue))
  (bind _returnvalue_3 (Class|KismetMathLibrary|DegAtan2 (.z _returnvalue_2) (.y _returnvalue_2)))
  (if (>= _returnvalue_3 0.0)
    (LocalVariables|SetResult_Local _returnvalue_3)
    (else
      (LocalVariables|SetResult_Local (Math|Float|MapRangeClamped _returnvalue_3 0.0 -1.8e+02 3.6e+02 1.8e+02))))
  (Math|Float|CompareFloat (LocalVariables|GetResult_Local) 9e+01
    (:>
      (Math|Float|CompareFloat (LocalVariables|GetResult_Local) 1.8e+02
        (:>
          (Math|Float|CompareFloat (LocalVariables|GetResult_Local) 2.7e+02
            (:>
              _)
            (:==
              _)
            (:<
              (return 3)))
          (return 4))
        (:<
          (return 2))))
    (:<
      (return 1))))